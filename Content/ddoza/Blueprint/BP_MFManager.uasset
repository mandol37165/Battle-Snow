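; Manager actor for the magnetic field zone, which currently only shows a periodic warning to the player.
; Tick runs through latent Delays to display WBP_MFWarning roughly every 30 seconds and remove it 2 seconds later.
; Disconnected, never-executed logic would spawn BP_MagneticField at a random BP_MFPoint and lerp its horizontal scale toward 10% smaller targets.
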(event `self.ReceiveBeginPlay`)

(event `self.ReceiveTick`
  (params (DeltaSeconds :type "Float (single-precision)"))
  (`KismetSystemLibrary.Delay` 30.0)
  (bind _returnvalue (`|CreateWidget` "/Game/ddoza/UI/WBP_MFWarning.WBP_MFWarning_C"))
  (`UserWidget.AddToViewport` _returnvalue 0)
  (`KismetSystemLibrary.Delay` 2.0)
  (`Widget.RemoveFromParent` _returnvalue))

(fn `UserConstructionScript`)