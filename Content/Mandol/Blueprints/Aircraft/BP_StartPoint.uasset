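; BP_StartPoint is a spawn marker that launches an aircraft on a straight path through a referenced center actor.
; On BeginPlay it rotates to face CenterRef and spawns a BP_StopPoint along that direction at twice the distance to the center, on the opposite side.
; It then spawns a BP_Aircraft at its own transform, passing the stop point's location as the destination along with a fixed speed.
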(event `self.ReceiveBeginPlay`
  (bind _defaultsceneroot (`self.DefaultSceneRoot`))
  (`SceneComponent.K2_SetWorldRotation` (`self.DefaultSceneRoot`) (`KismetMathLibrary.FindLookAtRotation` (`SceneComponent.K2_GetComponentLocation` (`self.DefaultSceneRoot`)) (`SceneComponent.K2_GetComponentLocation` (`/Game/Mandol/Blueprints/Aircraft/BP_CenterOfMap.DefaultSceneRoot` (`self.CenterRef`)))) false false)
  (set `self.ACDistance` (* (`self.GetDistanceTo` (`self.CenterRef`)) 2.0))
  (bind _returnvalue (`|SpawnActorFromClass` "/Game/Mandol/Blueprints/Aircraft/BP_StopPoint.BP_StopPoint_C" (`KismetMathLibrary.MakeTransform` (+ (`SceneComponent.K2_GetComponentLocation` _defaultsceneroot) (* (`KismetMathLibrary.GetForwardVector` (`SceneComponent.K2_GetComponentRotation` _defaultsceneroot)) (`self.ACDistance`)))) "Undefined" "MultiplyWithRoot" null null))
  (`|SpawnActorFromClass` "/Game/Mandol/Blueprints/Aircraft/BP_Aircraft.BP_Aircraft_C" (`SceneComponent.K2_GetComponentToWorld` (`self.DefaultSceneRoot`)) "AlwaysSpawn" "MultiplyWithRoot" null (`SceneComponent.K2_GetComponentLocation` (`/Game/Mandol/Blueprints/Aircraft/BP_StopPoint.DefaultSceneRoot` _returnvalue)) 0.06 null))

(fn `UserConstructionScript`)