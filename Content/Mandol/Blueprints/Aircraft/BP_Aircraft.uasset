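; C-130J transport aircraft actor that carries the player toward a destination and flags when they reach the jump position.
; BeginPlay caches the animation Blueprint and teleports player 0 to a random point around the spawn marker.
; Tick sweeps the plane toward ACDestination with a delta-scaled lerp, slowing as it nears.
; Custom events drive propeller and ramp animation, while ramp collision sets InJumpPos on overlapping BP_BSPlayer characters.
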(event `self.ReceiveBeginPlay`
  (bind _asabp_aircraft (cast `/Game/Mandol/Blueprints/Aircraft/ABP_Aircraft` (`SkeletalMeshComponent.GetAnimInstance` (`self.SK_West_Transport_C130J`))))
  (set `self.AnimInstance` _asabp_aircraft)
  (`self.K2_SetActorLocation` (`GameplayStatics.GetPlayerCharacter` 0) (`KismetMathLibrary.RandomPointInBoundingBox` (`SceneComponent.K2_GetComponentLocation` (`self.ACInSpawnPos`)) (400.0 80.0 1.0)) false false))

(event `self.ReceiveTick`
  (params (DeltaSeconds :type "Float (single-precision)"))
  (`self.K2_SetActorLocation` (`KismetMathLibrary.VLerp` (`self.K2_GetActorLocation`) (`self.ACDestination`) (* DeltaSeconds (`self.AircraftSpeed`))) true))

(event `SetPropellerSpeed`
  (params (PropellerSpeed :type "Float (double-precision)"))
  (set `/Game/Mandol/Blueprints/Aircraft/ABP_Aircraft.PropellerSpeed` (`KismetMathLibrary.MapRangeClamped` PropellerSpeed 0.0 1.0 0.0 1000.0) (`self.AnimInstance`)))

(event `OpenRamp`
  (params (OpenRampPosition :type "Float (double-precision)"))
  (set `/Game/Mandol/Blueprints/Aircraft/ABP_Aircraft.RampOpen` (`KismetMathLibrary.MapRangeClamped` OpenRampPosition 0.0 1.0 0.0 1.0) (`self.AnimInstance`)))

(event `self.RampCol.OnComponentBeginOverlap`
  (params (OverlappedComponent :type "PrimitiveComponent Object Reference") (OtherActor :type "Actor Object Reference") (OtherComp :type "PrimitiveComponent Object Reference") (OtherBodyIndex :type Integer) (bFromSweep :type Boolean) (SweepResult :type "HitResult Structure (by ref)"))
  (bind _asbp_bsplayer (cast `/Game/Mandol/Blueprints/BP_BSPlayer` OtherActor))
  (set `BSPlayer.inJumpPos` true _asbp_bsplayer))

(fn `UserConstructionScript`)