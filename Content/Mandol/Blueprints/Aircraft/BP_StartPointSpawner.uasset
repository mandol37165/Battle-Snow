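; Actor that spawns a BP_StartPoint at a randomized position around a center actor, then destroys itself.
; On Tick it orbits CenterRef at a random speed, rotating about an axis re-orthogonalized to the radius with cross products.
; After a zero-length delay it spawns the start point at its transform, passing CenterRef along.
; An invalid CenterRef triggers a short delayed retry.
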(event `self.ReceiveBeginPlay`
  (set `self.RSpeed` (`KismetMathLibrary.RandomFloatInRange` 1.0 999999.0)))

(event `Recheck`
  (bind _returnvalue (- (`SceneComponent.K2_GetComponentLocation` (`self.DefaultSceneRoot`)) (`self.PointToRotateAround`)))
  (`/Engine/EditorBlueprintResources/StandardMacros.IsValid` (`self.CenterRef`) :!label _label
    (:`Is Valid`
      (set `self.PointToRotateAround` (`SceneComponent.K2_GetComponentLocation` (`/Game/Mandol/Blueprints/Aircraft/BP_CenterOfMap.DefaultSceneRoot` (`self.CenterRef`))))
      (set `self.ACAxis` (`KismetMathLibrary.Normal` (`KismetMathLibrary.Cross_VectorVector` _returnvalue (`KismetMathLibrary.Cross_VectorVector` (`self.ACAxis`) _returnvalue))))
      (`self.K2_SetActorLocation` (`self.GetLoc`)))
    (:`Is Not Valid`
      (`KismetSystemLibrary.Delay` 0.01)
      (`self.Recheck`))))

(event `self.ReceiveTick`
  (params (DeltaSeconds :type "Float (single-precision)"))
  (set `self.Delta Seconds` DeltaSeconds)
  (`|ExecutionSequence`
    (:`then_0`
      (goto _label))
    (:`then_1`
      (`KismetSystemLibrary.Delay` 0.0)
      (`self.Started`))))

(event `Started`
  (bind _defaultsceneroot (`self.DefaultSceneRoot`))
  (`|SpawnActorFromClass` "/Game/Mandol/Blueprints/Aircraft/BP_StartPoint.BP_StartPoint_C" (`KismetMathLibrary.MakeTransform` (`SceneComponent.K2_GetComponentLocation` _defaultsceneroot) (`SceneComponent.K2_GetComponentRotation` _defaultsceneroot)) "Undefined" "MultiplyWithRoot" null (`self.CenterRef`) null)
  (`self.K2_DestroyActor`))

(fn `GetLoc`
  (returns (Loc :type "Vector Structure"))
  (return (+ (`KismetMathLibrary.RotateAngleAxis` (- (`SceneComponent.K2_GetComponentLocation` (`self.DefaultSceneRoot`)) (`self.PointToRotateAround`)) (* (`self.Delta Seconds`) (`self.RSpeed`)) (`self.ACAxis`)) (`self.PointToRotateAround`))))

(fn `UserConstructionScript`)