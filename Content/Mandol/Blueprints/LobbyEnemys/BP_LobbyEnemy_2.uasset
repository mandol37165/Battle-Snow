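; BP_LobbyEnemy_2 is a lobby enemy character that stands still until it sees a pawn, then chases and punches the player.
; Tick halts movement until pawn sensing, after a delay, sets IsPlayer and calls FollowPlayer.
; FollowPlayer moves to player 0 via AIMoveTo and, on arrival, plays a punch montage and sound.
; CanAttack gates the punch for the montage's duration but resets on each FollowPlayer call; no damage is applied here.
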(event `self.ReceiveTick`
  (params (DeltaSeconds :type "Float (single-precision)"))
  (if (not (`self.isPlayer`))
    (`MovementComponent.StopMovementImmediately` (`self.CharacterMovement`))))

(event `self.PawnSensing.OnSeePawn`
  (params (Pawn :type "Pawn Object Reference"))
  (`KismetSystemLibrary.Delay` 4.0)
  (set `self.isPlayer` true)
  (`self.FollowPlayer`))

(event `FollowPlayer`
  (set `self.canAttack` true)
  (if (`self.isPlayer`)
    (`|AIMoveTo` self (0.0 0.0 0.0) (`GameplayStatics.GetPlayerCharacter` 0) 70.0
      (:`OnSuccess`
        (if (`self.canAttack`)
          (set `self.canAttack` false)
          (bind _returnvalue (`self.PlayAnimMontage` "/Game/Mandol/Blueprints/LobbyEnemys/LEAnim/AM_Punching.AM_Punching"))
          (`GameplayStatics.PlaySound2D` "/Game/Sound/Kung_Fu_Old_School_Hit_04.Kung_Fu_Old_School_Hit_04" 1.0 1.0 0.0 null null)
          (`KismetSystemLibrary.Delay` _returnvalue)
          (set `self.canAttack` true))))
    (else
      (set `self.isPlayer` false))))

(fn `UserConstructionScript`)